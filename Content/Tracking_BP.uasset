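; Tracking actor that displays live population statistics for AI_Creature actors: count, average speed and average health.
; Every Tick it gathers all creatures with repeated GetAllActorsOfClass calls, sums Speed and FullHealth, and divides by the count.
; Results go to the PopCount, AvgMove and AvgHP texts, and the sums reset each frame.
; Average health uses truncated integer math, and neither division guards against an empty population.
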(event EventBeginPlay)

(event Collision|EventActorBeginOverlap
  (params (OtherActor :type Actor%20Object%20Reference)))

(event EventTick
  (params (DeltaSeconds :type Float%20%28single-precision%29))
  ;[1 1 1] Track Population
  (bind _outactors (Actor|GetAllActorsOfClass "/Game/AI_Creature.AI_Creature_C"))
  (Rendering|Components|TextRender|SetText (Variables|Default|GetPopCount) (Utilities|Text|ToText(Integer) (Utilities|Array|Length _outactors)))
  (Variables|Default|SetPopulation (Utilities|Array|Length _outactors))
  ;[1 1 1] Track Average Movement
  (bind _outactors_2 (Actor|GetAllActorsOfClass "/Game/AI_Creature.AI_Creature_C"))
  (for _array_element _outactors_2
    (Variables|Default|SetSpeedSum (+ (Variables|/Game/AI_Creature.AI_Creature_C|GetSpeed _array_element) (Variables|Default|GetSpeedSum))))
  (bind _output_get (Variables|Default|SetAverageSpeed (/ (Variables|Default|GetSpeedSum) (Math|Conversions|ToFloat(Integer) (Utilities|Array|Length _outactors)))))
  (Rendering|Components|TextRender|SetText (Variables|Default|GetAvgMove) (Utilities|Text|ToText(Float) _output_get "HalfToEven"))
  (Variables|Default|SetSpeedSum 0.0)
  (bind _outactors_3 (Actor|GetAllActorsOfClass "/Game/AI_Creature.AI_Creature_C"))
  (for _array_element_2 _outactors_3
    (Variables|Default|SetHealthSum (+ (Math|Float|Truncate (Variables|/Game/AI_Creature.AI_Creature_C|GetFullHealth _array_element_2)) (Variables|Default|GetHealthSum))))
  (bind _output_get_2 (Variables|Default|SetAverageHP (/ (Variables|Default|GetHealthSum) (Variables|Default|GetPopulation))))
  (Rendering|Components|TextRender|SetText (Variables|Default|GetAvgHP) (Utilities|Text|ToText(Integer) _output_get_2))
  (Variables|Default|SetHealthSum 0))

(fn ConstructionScript)